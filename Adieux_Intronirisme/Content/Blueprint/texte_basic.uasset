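; Actor that shows an editable line of 3D text in the world, always turned to face the player.
; The construction script applies the exposed string, size and color, the color through a dynamic instance of an unlit text material.
; Each Tick rotates the text component to look at the first player's character location.
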(event EventBeginPlay)

(event Collision|EventActorBeginOverlap
  (params (OtherActor :type Actor%20Object%20Reference)))

(event EventTick
  (params (DeltaSeconds :type Float%20%28single-precision%29))
  (Transformation|SetWorldRotation (Variables|Default|Gettext) (Math|Rotator|FindLookatRotation (Transformation|GetActorLocation) (Transformation|GetActorLocation (Game|GetPlayerCharacter 0))) false false))

(fn ConstructionScript
  (bind _text (Variables|Default|Gettext))
  (Rendering|Components|TextRender|SetText _text (Utilities|Text|ToText(String) (Variables|Default|Gettexte)))
  (bind _returnvalue (Rendering|Material|CreateDynamicMaterialInstance (Variables|Default|Gettext) 0 "/Game/Material/textUnlitMat.textUnlitMat" "None" :!class /Script/Engine.PrimitiveComponent))
  (Rendering|Material|SetVectorParameterValue _returnvalue "color" (Variables|Default|GettexteColor) :!class /Script/Engine.MaterialInstanceDynamic)
  (Rendering|Components|TextRender|SetWorldSize _text (Variables|Default|Getsize)))