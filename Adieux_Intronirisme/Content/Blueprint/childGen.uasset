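; Spawner Blueprint that periodically creates Child actors at a fixed line in the level, with slight random variation along X.
; Tick accumulates elapsed time and calls SpawnChild when the delay is reached, then re-rolls a short random delay.
; Each new Child gets a random Boy flag and a Parent reference to this spawner, then has Burn called on it.
; A separate Destroy function removes a given Child.
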(event EventTick
  (params (DeltaSeconds :type Float%20%28single-precision%29))
  (bind _output_get (Variables|Default|SetlastSpawn (+ DeltaSeconds (Variables|Default|GetlastSpawn))))
  (if (>= _output_get (Variables|Default|Getdelay))
    (CallFunction|SpawnChild)
    (Variables|Default|Setdelay (Math|Random|RandomFloatinRange 0.5 1.0))
    (Variables|Default|SetlastSpawn 0.0)))

(fn ConstructionScript)

(fn Destroy
  (params (child :type Child%20Object%20Reference))
  (Actor|DestroyActor child))

(fn SpawnChild
  (bind _returnvalue (Game|SpawnActorfromClass "/Game/Blueprint/child.child_C" (Math|Transform|MakeTransform (Math|Vector|MakeVector (Math|Random|RandomFloatinRange 615.0 7.1e+02) 1.05e+03 2.5e+02) "0,90.000000, 0") "Undefined" 0 0))
  (Variables|/Game/Blueprint/child.child_C|Setboy _returnvalue (Math|Random|RandomBool))
  (Variables|/Game/Blueprint/child.child_C|Setparent _returnvalue self)
  (Default|Burn _returnvalue))