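; Child Blueprint is a Paper2D sprite figure, either boy or girl, that animates and is removed when burned.
; The construction script picks the starting sprite from the Boy flag.
; The burn event plays the Travel timeline, which drives the sprite's relative location and uses an event track to swap to the gendered second sprite.
; When the timeline finishes, it passes itself to Parent's Destroy.
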(event Custom|burn
  (bind _papersprite (Variables|Default|GetPaperSprite))
  (bind _progress (Timeline|travel PlayFromStart)
    (:Update
      (Transformation|SetRelativeLocation (Variables|Default|GetPaperSprite) _progress false false))
    (:Finished
      (Default|Destroy (Variables|Default|Getparent) self))
    (:changeSprite
      (if (Variables|Default|Getboy)
        (Rendering|Components|Sprite|SetSprite _papersprite "/Game/Sprite/boyF_Sprite.boyF_Sprite")
        (else
          (Rendering|Components|Sprite|SetSprite _papersprite "/Game/Sprite/girlF_Sprite.girlF_Sprite"))))))

(fn ConstructionScript
  (bind _papersprite (Variables|Default|GetPaperSprite))
  (if (Variables|Default|Getboy)
    (Rendering|Components|Sprite|SetSprite _papersprite "/Game/Sprite/boyS_Sprite.boyS_Sprite")
    (else
      (Rendering|Components|Sprite|SetSprite _papersprite "/Game/Sprite/girlS_Sprite.girlS_Sprite"))))