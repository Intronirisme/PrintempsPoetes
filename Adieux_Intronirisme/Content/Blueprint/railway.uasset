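; Railway Blueprint that procedurally lays out a straight stretch of track from a configurable length.
; The construction script loops once per 400-unit segment along the local Y axis, up to the Lenght variable.
; Each step adds three static mesh components: one on the center line and one offset 170 units to either side in X.
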(fn ConstructionScript
  (for _index (range 0 (/ (Variables|Default|Getlenght) 400))
    (AddComponent|AddStaticMeshComponent false (Math|Transform|MakeTransform (* "0.000000,1.000000, 0" (* _index 400))))
    (AddComponent|AddStaticMeshComponent false (Math|Transform|MakeTransform (+ (* "0.000000,1.000000, 0" (* _index 400)) "170.000000,0.000000, 0")))
    (AddComponent|AddStaticMeshComponent false (Math|Transform|MakeTransform (+ (* "0.000000,1.000000, 0" (* _index 400)) "-170.000000,0.000000, 0")))))