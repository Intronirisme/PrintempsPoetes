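; An actor with a Plane component that toggles between visible, collidable and vanished, non-collidable states.
; The toogle event, gated by Activated, runs the Vanish timeline forward or in reverse to drive the Plane's "opacity" material parameter.
; Collision returns as soon as reappearing starts but turns off only when fading out finishes.
; The construction script disables shadow casting and applies the initial opacity and collision from Visible.
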(event Custom|toogle
  (if (Variables|Default|Getactivated)
    (if (Variables|Default|Getvisible)
      (Variables|Default|Setvisible false)
      (bind _opacity (Timeline|vanish Play)
        (:Update
          (Rendering|Material|SetScalarParameterValueonMaterials (Variables|Default|GetPlane) "opacity" _opacity))
        (:Finished
          (if (not (Variables|Default|Getvisible))
            (Collision|SetActorEnableCollision false))))
      (else
        (Variables|Default|Setvisible true)
        (Collision|SetActorEnableCollision true)
        (Timeline|vanish ReverseFromEnd)))))

(fn ConstructionScript
  (bind _plane (Variables|Default|GetPlane))
  (Rendering|SetCastShadow (Variables|Default|GetPlane) false)
  (if (Variables|Default|Getvisible)
    (Rendering|Material|SetScalarParameterValueonMaterials _plane "opacity" 1.0)
    (Collision|SetActorEnableCollision true)
    (else
      (Rendering|Material|SetScalarParameterValueonMaterials _plane "opacity" 0.0)
      (Collision|SetActorEnableCollision false))))