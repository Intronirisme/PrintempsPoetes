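; Player pawn with axis-driven walking and looking that detects texte actors in front of it.
; Forward and Right inputs move it along its own vectors scaled by WalkSpeed, while look inputs add controller yaw and pitch scaled by LookSensitivity.
; Every tick, a Visibility line trace runs from above the actor's origin along the player controller's forward vector and calls Focus on any texte actor hit.
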(event EventTick
  (params (DeltaSeconds :type Float%20%28single-precision%29))
  (bind _returnvalue (Transformation|GetActorLocation))
  (bind _returnvalue_2 (+ _returnvalue "0, 0,60.000000"))
  (bind (_outhit _returnvalue_3) (Collision|LineTraceByChannel _returnvalue_2 (+ _returnvalue_2 (* (Transformation|GetActorForwardVector (Game|GetPlayerController 0)) 3000)) "TraceTypeQuery1" false 0 "None"))
  (if _returnvalue_3
    (bind _astexte (Utilities|Casting|CastTotexte (.HitActor (Collision|BreakHitResult _outhit))))
    (Default|Focus _astexte)))

(event Input|AxisEvents|InputAxisForward
  (params (AxisValue :type Float%20%28single-precision%29))
  (Pawn|Input|AddMovementInput (Transformation|GetActorForwardVector) (* AxisValue (Variables|Default|GetwalkSpeed)) false))

(event Input|AxisEvents|InputAxisRight
  (params (AxisValue :type Float%20%28single-precision%29))
  (Pawn|Input|AddMovementInput (Transformation|GetActorRightVector) (* AxisValue (Variables|Default|GetwalkSpeed)) false))

(event Input|AxisEvents|InputAxisLookH
  (params (AxisValue :type Float%20%28single-precision%29))
  (Class|PlayerController|AddYawInput (Game|GetPlayerController 0) (* AxisValue (Variables|Default|GetlookSensitivity))))

(event Input|AxisEvents|InputAxisLookV
  (params (AxisValue :type Float%20%28single-precision%29))
  (Class|PlayerController|AddPitchInput (Game|GetPlayerController 0) (* AxisValue (Variables|Default|GetlookSensitivity))))

(fn ConstructionScript)