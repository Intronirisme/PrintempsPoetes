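; World text actor that turns to face the player and shrinks away once it has been read.
; Each focus call restarts a countdown and reverses the Vanish timeline; when it expires, the timeline scales the text size down, then hides the actor and disables collision.
; The first focus also calls TexteMan.Go, while hide and reveal events toggle visibility and collision.
; The construction script applies text, color, size and plane scale.
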(event Custom|focus
  (bind _text (Variables|Default|Gettext))
  (if (Variables|Default|GetreadedFirst)
    _
    (else
      (Default|Go (Variables|Default|GettexteMan))))
  (Variables|Default|Setis_focus 1.0)
  (Variables|Default|Setreaded true)
  (Variables|Default|SetreadedFirst true)
  (bind _opacity (Timeline|vanish Reverse)
    (:Update
      (Rendering|Components|TextRender|SetWorldSize _text (* _opacity (Variables|Default|Getsize))))
    (:Finished
      (if (<= (Variables|/Script/Engine.TextRenderComponent|GetWorldSize _text) 0.1)
        (Rendering|SetActorHiddenInGame true)
        (Collision|SetActorEnableCollision false)))))

(event Custom|hide
  (Rendering|SetActorHiddenInGame true)
  (Collision|SetActorEnableCollision false))

(event Custom|reveal
  (Rendering|SetActorHiddenInGame false)
  (Collision|SetActorEnableCollision true))

(event EventTick
  (params (DeltaSeconds :type Float%20%28single-precision%29))
  (bind _text (Variables|Default|Gettext))
  (Variables|Default|Setis_focus (Math|Float|Clamp(Float) (- (Variables|Default|Getis_focus) DeltaSeconds) 0.0 3.0))
  (Transformation|SetWorldRotation (Variables|Default|Gettext) (Math|Rotator|FindLookatRotation (Transformation|GetActorLocation) (Transformation|GetActorLocation (Game|GetPlayerCharacter 0))) false false)
  (if (and (Variables|Default|Getreaded) (== (Variables|Default|Getis_focus) 0.0))
    (Variables|Default|Setreaded false)
    (bind _opacity (Timeline|vanish PlayFromStart)
      (:Update
        (Rendering|Components|TextRender|SetWorldSize _text (* _opacity (Variables|Default|Getsize))))
      (:Finished
        (if (<= (Variables|/Script/Engine.TextRenderComponent|GetWorldSize _text) 0.1)
          (Rendering|SetActorHiddenInGame true)
          (Collision|SetActorEnableCollision false))))))

(fn ConstructionScript
  (bind _text (Variables|Default|Gettext))
  (Rendering|Components|TextRender|SetText _text (Utilities|Text|ToText(String) (Variables|Default|Gettexte)))
  (bind _returnvalue (Rendering|Material|CreateDynamicMaterialInstance _text 0 "/Game/Material/textUnlitMat.textUnlitMat" "None" :!class /Script/Engine.PrimitiveComponent))
  (Rendering|Material|SetVectorParameterValue _returnvalue "color" (Variables|Default|GettexteColor) :!class /Script/Engine.MaterialInstanceDynamic)
  (Rendering|Components|TextRender|SetWorldSize _text (Variables|Default|Getsize))
  (Transformation|SetRelativeScale3D (Variables|Default|GetPlane) (Math|Vector|MakeVector (Variables|Default|GetscaleX) (Variables|Default|GetscaleY) 1.0)))