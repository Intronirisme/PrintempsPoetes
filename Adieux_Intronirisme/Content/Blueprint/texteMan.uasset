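; texteMan is a manager Blueprint that reveals the text objects in LsTxt one at a time.
; Each call to the go event reveals the next entry and advances index I.
; Once all are revealed, further calls teleport the last entry and Player 6000 units along Y.
; The construction script hides every entry when Ready is set and reveals them otherwise.
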(event Custom|go
  (bind _lstxt (Variables|Default|GetlsTxt))
  (if (== (Variables|Default|Geti) (Utilities|Array|Length _lstxt))
    (Transformation|AddActorWorldOffset (Utilities|Array|Get(acopy) (Variables|Default|GetlsTxt) (- (Variables|Default|Geti) 1)) "0,6000.000000, 0" false true)
    (Transformation|AddActorWorldOffset (Variables|Default|Getplayer) "0,6000.000000, 0" false true)
    (else
      (Default|Reveal (Utilities|Array|Get(acopy) _lstxt (Variables|Default|Geti)))
      (Variables|Default|Seti (+ (Variables|Default|Geti) 1)))))

(fn ConstructionScript
  (if (Variables|Default|Getready)
    (for _array_element (Variables|Default|GetlsTxt)
      (Default|Hide _array_element))
    (else
      (for _array_element_2 (Variables|Default|GetlsTxt)
        (Default|Reveal _array_element_2)))))