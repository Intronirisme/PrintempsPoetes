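; Wagon actor that closes its doors, travels a set distance sideways, then reopens them after a short pause.
; A timeline slides two door meshes in mirrored directions, and closing reverses it behind a one-shot guard.
; Tick linearly moves the actor along its negative right vector, toward the end point the construction script marks on a spline.
; Vanish events swap body and door materials to transparent, while unvanish restores some body materials.
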(event Custom|openDoor
  (bind _posporte (Timeline|ouverture Play)
    (:Update
      (Transformation|SetRelativeLocation (Variables|Default|GetStaticMesh3) _posporte false false)
      (Transformation|SetRelativeLocation (Variables|Default|GetStaticMesh2) (Math|Vector|MakeVector (.X (Math|Vector|BreakVector _posporte)) (* -1 (.Y (Math|Vector|BreakVector _posporte))) (.Z (Math|Vector|BreakVector _posporte))) false false))))

(event Custom|closeDoor
  (if (Variables|Default|GetcanCloseAgain)
    (Variables|Default|SetcanCloseAgain false)
    (Rendering|Material|SetMaterial (Variables|Default|GetStaticMesh3) 1 "/Game/Material/black.black")
    (Rendering|Material|SetMaterial (Variables|Default|GetStaticMesh2) 1 "/Game/Material/black.black")
    (bind _posporte (Timeline|ouverture Reverse)
      (:Update
        (Transformation|SetRelativeLocation (Variables|Default|GetStaticMesh3) _posporte false false)
        (Transformation|SetRelativeLocation (Variables|Default|GetStaticMesh2) (Math|Vector|MakeVector (.X (Math|Vector|BreakVector _posporte)) (* -1 (.Y (Math|Vector|BreakVector _posporte))) (.Z (Math|Vector|BreakVector _posporte))) false false)))))

(event Custom|start
  (CallFunction|CloseDoor)
  (Utilities|FlowControl|Delay 3.0)
  (Variables|Default|Setmoving true))

(event Custom|vanish
  (bind _staticmesh (Variables|Default|GetStaticMesh))
  (Rendering|Material|SetMaterial _staticmesh 0 "/Game/Material/transp.transp")
  (Rendering|Material|SetMaterial _staticmesh 1 "/Game/Material/transp.transp")
  (Rendering|Material|SetMaterial _staticmesh 2 "/Game/Material/transp.transp")
  (Rendering|Material|SetMaterial _staticmesh 3 "/Game/Material/transp.transp")
  (for _array_element (Variables|Default|GetlsDoor)
    (Rendering|Material|SetMaterial _array_element 1 "/Game/Material/transp.transp"))
  (Rendering|Material|SetMaterial (Variables|Default|GetStaticMesh2) 1 "/Game/Material/transp.transp")
  (Rendering|Material|SetMaterial (Variables|Default|GetStaticMesh3) 1 "/Game/Material/transp.transp"))

(event Custom|unvanish
  (bind _staticmesh (Variables|Default|GetStaticMesh))
  (Rendering|Material|SetMaterial _staticmesh 0 "/Engine/BasicShapes/BasicShapeMaterial.BasicShapeMaterial")
  (Rendering|Material|SetMaterial _staticmesh 2 "/Engine/MapTemplates/Materials/BasicAsset01.BasicAsset01")
  (Rendering|Material|SetMaterial _staticmesh 3 "/Engine/EditorMeshes/ColorCalibrator/M_ClearCoatBlack.M_ClearCoatBlack"))

(event EventTick
  (params (DeltaSeconds :type Float%20%28single-precision%29))
  (if (Variables|Default|Getmoving)
    (Variables|Default|Setprogress (+ DeltaSeconds (Variables|Default|Getprogress)))
    (Transformation|SetActorLocation (+ (Variables|Default|Getorigin) (* (* (Transformation|GetActorRightVector) -1) (* (/ (Variables|Default|Getprogress) (Variables|Default|Gettime)) (Variables|Default|Getdistance)))) false false)
    (if (>= (Variables|Default|Getprogress) (Variables|Default|Gettime))
      (Variables|Default|Setmoving false)
      (Utilities|FlowControl|Delay 2.0)
      (CallFunction|OpenDoor))))

(fn ConstructionScript
  (Variables|Default|SetlsDoor (Utilities|Array|MakeArray (Variables|Default|GetStaticMesh0) (Variables|Default|GetStaticMesh1) (Variables|Default|GetStaticMesh4) (Variables|Default|GetStaticMesh5) (Variables|Default|GetStaticMesh6) (Variables|Default|GetStaticMesh7) (Variables|Default|GetStaticMesh8) (Variables|Default|GetStaticMesh9) (Variables|Default|GetStaticMesh10) (Variables|Default|GetStaticMesh11) (Variables|Default|GetStaticMesh)))
  (Variables|Default|Setorigin (Transformation|GetWorldLocation (Variables|Default|GetStaticMesh)))
  (Spline|SetLocationatSplinePoint (Variables|Default|GetSpline) 0 (+ (* (* (Transformation|GetActorRightVector) -1) (Variables|Default|Getdistance)) (Variables|Default|Getorigin)) "World" true))